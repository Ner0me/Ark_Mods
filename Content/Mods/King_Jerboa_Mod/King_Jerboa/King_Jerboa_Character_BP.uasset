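; King Jerboa creature Blueprint that warns nearby players of incoming weather with alert animations.
; On a randomized interval while conscious, its server timer reads the day cycle manager's warning for rain, sandstorm, superheat or electrical storm.
; It skips alerts when a valid Target is on another team, and requires a player pawn nearby via an octree query.
; Each warning event plays a riding or standard montage depending on IsMounted.
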(event `PlayWeatherWarning_Rain`
  (`self.PlayAnimEx` (select `bool` (`self.bIsMounted`) :`false` "/Game/ScorchedEarth/Dinos/Jerboa/Animations/Jerboa-Alert-Rainstorm_Montage.Jerboa-Alert-Rainstorm_Montage" :`true` "/Game/ScorchedEarth/Dinos/Jerboa/Animations/Jerboa-Riding-Alert-Rainstorm_Montage.Jerboa-Riding-Alert-Rainstorm_Montage" :!type "AnimMontage Object Reference") 1.0 "None" false false false true))

(event `PlayWeatherWarning_Superheat`
  (`self.PlayAnimEx` (select `bool` (`self.bIsMounted`) :`false` "/Game/ScorchedEarth/Dinos/Jerboa/Animations/Jerboa-Alert-Heatwave_Montage.Jerboa-Alert-Heatwave_Montage" :`true` "/Game/ScorchedEarth/Dinos/Jerboa/Animations/Jerboa-Riding-Alert-Heatwave_Montage.Jerboa-Riding-Alert-Heatwave_Montage" :!type "AnimMontage Object Reference") 1.0 "None" false false false true))

(event `PlayWeatherWarning_ElectricalStorm`
  (`self.PlayAnimEx` (select `bool` (`self.bIsMounted`) :`false` "/Game/ScorchedEarth/Dinos/Jerboa/Animations/Jerboa-Alert-Electricalstorm_Montage.Jerboa-Alert-Electricalstorm_Montage" :`true` "/Game/ScorchedEarth/Dinos/Jerboa/Animations/Jerboa-Riding-Alert-Electricalstorm_Montage.Jerboa-Riding-Alert-Electricalstorm_Montage" :!type "AnimMontage Object Reference") 1.0 "None" false false false true))

(event `PlayWeatherWarning_Sandstorm`
  (`self.PlayAnimEx` (select `bool` (`self.bIsMounted`) :`false` "/Game/ScorchedEarth/Dinos/Jerboa/Animations/Jerboa-Alert-Sandstorm_Montage.Jerboa-Alert-Sandstorm_Montage" :`true` "/Game/ScorchedEarth/Dinos/Jerboa/Animations/Jerboa-Riding-Alert-Sandstorm_Montage.Jerboa-Riding-Alert-Sandstorm_Montage" :!type "AnimMontage Object Reference") 1.0 "None" false false false true))

(fn `BPTimerServer`
  (bind _returnvalue (`self.K2_GetWorld`))
  (bind _bnearby (`self.IsPlayerNearby`))
  (bind _target (`self.Target`))
  (if (`self.BPIsConscious`)
    (if (`VictoryCore.IsTimeSince` _returnvalue (`self.LastAlertAnimTime`) (`KismetMathLibrary.RandomFloatInRange` (`self.AlertIntervalMin`) (`self.AlertIntervalMax`)))
      (set `self.LastAlertAnimTime` (`KismetSystemLibrary.GetGameTimeInSeconds`))
      (if (`KismetSystemLibrary.IsValid` _target)
        (if (== (`Actor.TargetingTeam` _target) (`self.TargetingTeam`))
          (bind _returnvalue_2 (`PrimalGlobals.GetDayCycleManager` _returnvalue :!label _label))
          (bind _asdaycyclemanagerbase_c (cast `/Game/PrimalEarth/CoreBlueprints/DayCycleManagerBase` _returnvalue_2))
          (bind _weathereventwarningtype (`/Game/PrimalEarth/CoreBlueprints/DayCycleManagerBase.GetWeatherEventWarning` _asdaycyclemanagerbase_c))
          (switch `int` _weathereventwarningtype
            (:`1`
              (if _bnearby
                (`self.PlayWeatherWarning_Rain`)))
            (:`2`
              (if _bnearby
                (`self.PlayWeatherWarning_Sandstorm`)))
            (:`3`
              (if _bnearby
                (`self.PlayWeatherWarning_Superheat`)))
            (:`4`
              (if _bnearby
                (`self.PlayWeatherWarning_ElectricalStorm`)))))
        (else
          (goto _label))))))

(fn `IsPlayerNearby`
  (returns (bNearby :type Boolean))
  (bind _returnvalue (`VictoryCore.ServerOctreeOverlapActors` (`self.K2_GetWorld`) (`self.K2_GetActorLocation`) 5500.0 "PLAYERPAWNS"))
  (return (> (`KismetArrayLibrary.Array_Length` _returnvalue) 0)))

(fn `UserConstructionScript`
  (`parent.UserConstructionScript`))