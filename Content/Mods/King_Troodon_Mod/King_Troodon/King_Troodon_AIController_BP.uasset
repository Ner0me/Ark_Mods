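; AI controller for the King Troodon mod creature, overriding targeting desire to make wild Troodons hunt according to pack strength.
; Humans get a desire multiplier, but wild Troodons reject them without aggro beyond a fraction of natural targeting range.
; Other creatures too heavy to drag are rejected unless over two same-team Troodons are nearby or the Troodon was recently hurt.
; A lone Troodon also attacks heavy targets at close range.
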(fn `BPGetTargetingDesire`
  (params (ForTarget :type "Actor Object Reference") (ForTargetingDesireValue :type "Float (double-precision)"))
  (returns (ReturnValue :type "Float (double-precision)"))
  (bind _returnvalue (`self.K2_GetPawn`))
  (set `self.ReturnVal` ForTargetingDesireValue)
  (bind _asprimalcharacter (cast `PrimalCharacter` ForTarget)
    (:`then`
      (bind _returnvalue_2 (`self.IsShooterCharacter` _asprimalcharacter))
      (if _returnvalue_2
        (set `self.ReturnVal` (* ForTargetingDesireValue (`self.AttackHumanDesireMultiplier`)))
        (else
          (bind _asprimaldinocharacter (cast `PrimalDinoCharacter` _returnvalue)
            (:`then`
              (if (`PrimalDinoCharacter.BPIsTamed` _asprimaldinocharacter)
                _
                (elif (not (or (`PrimalCharacter.bIsDead` _asprimalcharacter) (< (`KismetMathLibrary.Conv_DoubleToFloat` (- (`KismetSystemLibrary.GetGameTimeInSeconds`) (`PrimalCharacter.LastTookDamageTime` _asprimaldinocharacter))) (`self.TimeAggressiveAfterTakingDamage`))))
                  (bind _asshootergamemode (cast `ShooterGameMode` (`GameplayStatics.GetGameMode`))
                    (:`then`
                      (bind _returnvalue_3 (`ShooterGameMode.CountOverlappingDinoCharactersOfTeamAndClass` _asshootergamemode (`self.K2_GetActorLocation` _asprimaldinocharacter) (`self.AggroNotifyNeighborsRange`) "/Game/Mods/King_Troodon_Mod/King_Troodon/King_Troodon_Character_BP.King_Troodon_Character_BP_C" (`self.TargetingTeam`) true false))
                      (if (> _returnvalue_3 2)
                        _
                        (elif (> _returnvalue_3 1)
                          (bind _returnvalue_4 (`PrimalCharacter.GetDragWeight` _asprimalcharacter null :!label _label))
                          (bind _returnvalue_5 (`self.IsShooterCharacter` _asprimalcharacter))
                          (if (not (or (and (> (`self.MaxDragWeightToAttackSolo`) _returnvalue_4) (not _returnvalue_5)) _returnvalue_5))
                            (set `self.ReturnVal` -1.0))
                          (elif (< (`KismetMathLibrary.VSize` (- (`self.K2_GetActorLocation` _asprimalcharacter) (`self.K2_GetActorLocation` (`self.K2_GetPawn`)))) (`self.AllowAttackingIfThisCloseDistance`))
                            _
                            (else
                              (goto _label))))))
                    (:`CastFailed`
                      _)))))
            (:`CastFailed`
              _)))))
    (:`CastFailed`
      _))
  (`|ExecutionSequence`
    (:`then_0`
      (if _returnvalue_2
        (bind _asprimaldinocharacter_2 (cast `PrimalDinoCharacter` (`self.K2_GetPawn`)))
        (if (not (`PrimalDinoCharacter.BPIsTamed` _asprimaldinocharacter_2))
          (bind _returnvalue_6 (`self.GetAggroDesirability` ForTarget))
          (if (<= _returnvalue_6 0.0)
            (if (> (`KismetMathLibrary.VSize` (- (`self.K2_GetActorLocation` ForTarget) (`self.K2_GetActorLocation` _returnvalue))) (`KismetMathLibrary.FMax` (* (`self.NaturalTargetingRange`) 0.54) 395.0))
              (set `self.ReturnVal` -1.0))))))
    (:`then_1`
      (return (`self.ReturnVal`)))))

(fn `UserConstructionScript`
  (`parent.UserConstructionScript`))