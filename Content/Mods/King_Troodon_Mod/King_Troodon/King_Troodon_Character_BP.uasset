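; King Troodon creature character that grows more dangerous at night, with wider-or-narrower aggro ranges, pack bonus and glowing eyes switched by the day cycle.
; Wild ones tame by killing a tribe's tamed creatures; tamed ones share kill XP with nearby allies.
; Radial-menu scouting triggers server octree scans, multicast to nearby teammates as pulsing HUD icons, with range and recharge upgraded by spending level-ups.
; Jumps at enemy targets become slope-aligned pounces.
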(event Custom|NetDisplaySonar
  (params (SonarType :type Integer) (SonarPoints :type Array%20of%20Vectors))
  (bind _returnvalue (Game|GetPlayerController 0))
  (if (not (Networking|IsDedicatedServer))
    (if (and (< (Math|Vector|VectorLength (- (Camera|GetCameraLocation (Variables|/Script/Engine.PlayerController|GetPlayerCameraManager _returnvalue)) (Transformation|GetActorLocation))) (Variables|Sonar|GetSonarViewRange)) (== (Variables|/Script/Engine.Actor|GetTargetingTeam _returnvalue) (Variables|Default|GetTargetingTeam)))
      (Utilities|Array|SetArrayElem (Variables|Sonar|GetSonarDisplayTimes) SonarType (Utilities|Time|GetGameTimeinSeconds) true)
      (switch int SonarType
        (:0
          (Variables|Sonar|SetSonarPointsType0 SonarPoints))
        (:1
          (Variables|Sonar|SetSonarPointsType1 SonarPoints))
        (:2
          (Variables|Sonar|SetSonarPointsType2 SonarPoints))
        (:3
          (Variables|Sonar|SetSonarPointsType3 SonarPoints)))
      (if (> (Utilities|Array|Length SonarPoints) 0)
        (Class|PrimalCharacter|PlayAnimEx "/Game/PrimalEarth/Dinos/Troodon/Animations/Troodon-Spot_Montage.Troodon-Spot_Montage" 1.0 "None" true true false false)))))

(event Custom|AnimNotify_DoSonar
  (if (Networking|IsServer)
    ;[1 1 1] To add a wait time between the anims. Placed here so the found anim will be more accurate
    (Utilities|FlowControl|Delay 1.0)
    (CallFunction|DoSonar (Variables|Sonar|GetSonarMode))))

(event Custom|Net%20Update%20Last%20Time%20Sonar%20Used
  (Variables|Sonar|SetLastTimeSonarWasUsed (Utilities|Time|GetGameTimeinSeconds)))

(event EventBeginPlay
  (bind _nighteyes (Variables|FX|GetNightEyes))
  (bind _nightnotifyneighborrange (Variables|Default|GetNightNotifyNeighborRange))
  (bind _daynotifyneighborrange (Variables|Default|GetDayNotifyNeighborRange))
  (bind _daytimetargetingrange (Variables|Default|GetDayTimeTargetingRange))
  (bind _nighttimetargetingrange (Variables|Default|GetNightTimeTargetingRange))
  (Variables|Taming|SetLastTimeRecievedAffinity -6e+01)
  (bind _asking_troodon_aicontroller_bp_c (Utilities|Casting|CastToKing_Troodon_AIController_BP (Pawn|GetController)))
  (bind _returnvalue (Class|PrimalGlobals|GetDayCycleManager (Class|Actor|GetWorld)))
  (bind _returnvalue_2 (Class|DayCycleManager|IsDaytime _returnvalue))
  (if _returnvalue_2
    (Variables|/Script/ShooterGame.PrimalDinoAIController|SetNaturalTargetingRange _asking_troodon_aicontroller_bp_c _daytimetargetingrange)
    (Variables|/Script/ShooterGame.PrimalDinoAIController|SetAggroNotifyNeighborsRange _asking_troodon_aicontroller_bp_c _daynotifyneighborrange)
    (Variables|/Script/ShooterGame.PrimalDinoAIController|SetTamedTargetingRange _asking_troodon_aicontroller_bp_c _daytimetargetingrange)
    (Variables|Default|SetDamageNotifyTeamAggroRange _daynotifyneighborrange)
    (Variables|Default|SetbUseGang false)
    (Components|Activation|SetActive _nighteyes false true)
    (else
      (Variables|/Script/ShooterGame.PrimalDinoAIController|SetNaturalTargetingRange _asking_troodon_aicontroller_bp_c _nighttimetargetingrange)
      (Variables|/Script/ShooterGame.PrimalDinoAIController|SetAggroNotifyNeighborsRange _asking_troodon_aicontroller_bp_c _nightnotifyneighborrange)
      (Variables|/Script/ShooterGame.PrimalDinoAIController|SetTamedTargetingRange _asking_troodon_aicontroller_bp_c _nighttimetargetingrange)
      (Variables|Default|SetDamageNotifyTeamAggroRange _nightnotifyneighborrange)
      (Variables|Default|SetbUseGang true)
      (if (not (Networking|IsDedicatedServer))
        (Components|Activation|SetActive _nighteyes true true)))))

(fn ConstructionScript
  (|CallParentFunction))

(fn BPKilledSomethingEvent
  (params (killedTarget :type Primal%20Character%20Object%20Reference))
  (bind _returnvalue (Class|PrimalDinoCharacter|BPIsTamed))
  (if (Networking|IsServer)
    (Utilities|FlowControl|Sequence
      (:then_0
        (if (Class|PrimalDinoCharacter|BPIsTamed)
          (Utilities|IsValid (Variables|/Script/ShooterGame.PrimalCharacter|GetMyCharacterStatusComponent killedTarget)
            (:Is%20Valid
              (if (Ability|HasAuthority)
                (bind _returnvalue_2 (Class|VictoryCore|ServerOctreeOverlapActors (Class|Actor|GetWorld) (Transformation|GetActorLocation) (Variables|Default|GetGiveAlliesXPRange) "PAWNS"))
                (for _array_element _returnvalue_2
                  (bind _asprimalcharacter (Utilities|Casting|CastToPrimalCharacter _array_element))
                  (if (not (== _asprimalcharacter self))
                    (if (and (not (Variables|/Script/ShooterGame.PrimalCharacter|GetbIsDead _asprimalcharacter)) (== (Variables|/Script/Engine.Actor|GetTargetingTeam _asprimalcharacter) (Variables|Default|GetTargetingTeam)))
                      (bind _returnvalue_3 (Class|PrimalCharacter|GetKillXP))
                      (Class|PrimalCharacterStatusComponent|AddExperience (Variables|/Script/ShooterGame.PrimalCharacter|GetMyCharacterStatusComponent _asprimalcharacter) (* _returnvalue_3 (Variables|Default|GetRatioOfXPOfKilledToGiveToAllies)) false "XP_KILL")))))))))
      (:then_1
        (bind _returnvalue_4 (Class|VictoryCore|StaticGetTimeSince (Class|Actor|GetWorld) (Variables|Taming|GetLastTimeRecievedAffinity)))
        (if (>= _returnvalue_4 (Variables|Taming|GetCooldownBeforeRecievingAffinity))
          (bind _returnvalue_5 (Class|PrimalCharacter|GetKillXP killedTarget))
          (bind _returnvalue_6 (Class|PrimalGlobals|GetDayCycleManager (Class|Actor|GetWorld)))
          (bind _returnvalue_7 (Class|DayCycleManager|IsDaytime _returnvalue_6))
          (LocalVariables|SetTamingAmount (Math|Float|SelectFloat (* (+ (* _returnvalue_5 (Variables|Taming|GetTamingAffinityMultiplier)) (Variables|Taming|GetBaseTamingAffinity)) (Variables|Default|GetDayTimeAffinityMultiplier)) (+ (* _returnvalue_5 (Variables|Taming|GetTamingAffinityMultiplier)) (Variables|Taming|GetBaseTamingAffinity)) _returnvalue_7))
          (if (<= (Variables|Default|GetCurrentTameAffinity) 0.0)
            (Variables|Default|SetTamingTeamID 0 false)
            (if _returnvalue
              _
              (else
                (Class|PrimalDinoCharacter|NetUpdateDinoNameStrings))))
          (if (not _returnvalue)
            (Class|PrimalCharacterStatusComponent|ModifyCurrentStatusValue (Variables|Default|GetMyCharacterStatusComponent) "Food" (Variables|Taming|GetFoodToGetPerKillWhileTaming) false false false false 0 false)
            (Utilities|FlowControl|Sequence
              (:then_0
                (bind _asprimaldinocharacter (Utilities|Casting|CastToPrimalDinoCharacter killedTarget))
                (if (and (!= (Variables|/Script/ShooterGame.PrimalDinoCharacter|GetTamedAggressionLevel _asprimaldinocharacter) 0) (not (Variables|Default|GetTargetHasARider)))
                  (if (== 0 (Variables|Default|GetTamingTeamID))
                    (bind _asprimaldinocharacter_2 (Utilities|Casting|CastToPrimalDinoCharacter killedTarget))
                    (if (Class|PrimalDinoCharacter|BPIsTamed _asprimaldinocharacter_2)
                      (Variables|Default|SetTamingTeamID (Variables|/Script/Engine.Actor|GetTargetingTeam _asprimaldinocharacter_2) false)
                      (Variables|Default|SetCurrentTameAffinity (+ (Variables|Default|GetCurrentTameAffinity) (LocalVariables|GetTamingAmount)) false)
                      (Class|PrimalDinoCharacter|NetUpdateDinoNameStrings (Utilities|String|SelectString (Variables|/Script/ShooterGame.PrimalCharacter|GetTribeName _asprimaldinocharacter_2) (Variables|/Script/ShooterGame.PrimalDinoCharacter|GetTamerString _asprimaldinocharacter_2) (> (Utilities|String|Len (Variables|/Script/ShooterGame.PrimalCharacter|GetTribeName _asprimaldinocharacter_2)) 0)))
                      (Variables|Taming|SetLastTimeRecievedAffinity (Utilities|Time|GetGameTimeinSeconds))
                      (if (not (Variables|Default|GetbIsWakingTame))
                        (Variables|Default|SetbIsWakingTame true false)))
                    (else
                      (bind _asprimaldinocharacter_3 (Utilities|Casting|CastToPrimalDinoCharacter killedTarget))
                      (if (Class|PrimalDinoCharacter|BPIsTamed _asprimaldinocharacter_3)
                        (if (== (Variables|/Script/Engine.Actor|GetTargetingTeam _asprimaldinocharacter_3) (Variables|Default|GetTamingTeamID))
                          (Variables|Default|SetCurrentTameAffinity (+ (Variables|Default|GetCurrentTameAffinity) (LocalVariables|GetTamingAmount)) false)
                          (Variables|Taming|SetLastTimeRecievedAffinity (Utilities|Time|GetGameTimeinSeconds))
                          (if (not (Variables|Default|GetbIsWakingTame))
                            (Variables|Default|SetbIsWakingTame true false))))))))
              (:then_1
                (if (>= (Variables|Default|GetCurrentTameAffinity) (Variables|Default|GetRequiredTameAffinity))
                  (Class|PrimalDinoCharacter|TameDino)
                  (Class|PrimalCharacter|PlayAnimEx "/Game/PrimalEarth/Dinos/Troodon/Animations/Troodon-Spot_Montage.Troodon-Spot_Montage" 1.0 "None" true false false false))))))))))

(fn BPTimerServer
  (bind _nightnotifyneighborrange (Variables|Default|GetNightNotifyNeighborRange))
  (bind _daynotifyneighborrange (Variables|Default|GetDayNotifyNeighborRange))
  (bind _daytimetargetingrange (Variables|Default|GetDayTimeTargetingRange))
  (bind _nighttimetargetingrange (Variables|Default|GetNightTimeTargetingRange))
  (if (Networking|IsServer)
    (bind _astroodon_aicontroller_bp_c (Utilities|Casting|CastToTroodon_AIController_BP (Pawn|GetController)))
    (bind _returnvalue (Class|PrimalGlobals|GetDayCycleManager (Class|Actor|GetWorld)))
    (bind _returnvalue_2 (Class|DayCycleManager|IsDaytime _returnvalue))
    (if _returnvalue_2
      (Variables|/Script/ShooterGame.PrimalDinoAIController|SetNaturalTargetingRange _astroodon_aicontroller_bp_c _daytimetargetingrange)
      (Variables|/Script/ShooterGame.PrimalDinoAIController|SetAggroNotifyNeighborsRange _astroodon_aicontroller_bp_c _daynotifyneighborrange)
      (Variables|/Script/ShooterGame.PrimalDinoAIController|SetTamedTargetingRange _astroodon_aicontroller_bp_c _daytimetargetingrange)
      (Variables|Default|SetDamageNotifyTeamAggroRange _daynotifyneighborrange)
      (Variables|Default|SetbUseGang false)
      (if (!= (Variables|Default|GetGangCount) 0)
        (Variables|Default|SetGangCount 0 false))
      (if (Variables|FX|GetEyesActivated)
        (Variables|FX|SetEyesActivated false false))
      (else
        (Variables|/Script/ShooterGame.PrimalDinoAIController|SetNaturalTargetingRange _astroodon_aicontroller_bp_c _nighttimetargetingrange)
        (Variables|/Script/ShooterGame.PrimalDinoAIController|SetAggroNotifyNeighborsRange _astroodon_aicontroller_bp_c _nightnotifyneighborrange)
        (Variables|/Script/ShooterGame.PrimalDinoAIController|SetTamedTargetingRange _astroodon_aicontroller_bp_c _nighttimetargetingrange)
        (Variables|Default|SetDamageNotifyTeamAggroRange _nightnotifyneighborrange)
        (Variables|Default|SetbUseGang true)
        (if (not (Variables|FX|GetEyesActivated))
          (Variables|FX|SetEyesActivated true false))))))

(fn OnRepEyesActivated
  (if (Variables|FX|GetEyesActivated)
    (if (not (Networking|IsDedicatedServer))
      (Components|Activation|SetActive (Variables|FX|GetNightEyes) true true))
    (else
      (Components|Activation|SetActive (Variables|FX|GetNightEyes) false true))))

(fn OnJumped
  (bind _returnvalue (Transformation|GetActorLocation))
  (bind _target (Variables|Default|GetTarget))
  (bind (_x _y _z) (Math|Vector|BreakVector _returnvalue))
  (bind (_x_2 _y_2 _z_2) (Math|Vector|BreakVector _returnvalue))
  (Utilities|IsValid _target
    (:Is%20Valid
      (if (!= (Variables|/Script/Engine.Actor|GetTargetingTeam _target) (Variables|Default|GetTargetingTeam))
        (Variables|Default|SetbStopMovementOnLanding true)
        (bind (_outhit _returnvalue_2) (Collision|LineTraceByChannel (Math|Vector|MakeVector _x_2 _y_2 _z_2) (Math|Vector|MakeVector _x _y (- _z 1e+03)) "ECC_WorldStatic" false 0 "None"))
        (bind _returnvalue_3 (CallFunction|BPGetAddForwardVelocityonJump))
        (Class|PrimalCharacter|BPNetAddCharacterMovementImpulse (* (Math|Vector|MakeVector (.X (Math|Vector|BreakVector (Math|Vector|SelectVector (Math|Vector|Normalize (* (Math|Vector|CrossProduct (.ImpactNormal (Collision|BreakHitResult _outhit)) (Transformation|GetActorRightVector)) -1.0)) (Transformation|GetActorForwardVector) _returnvalue_2))) (.Y (Math|Vector|BreakVector (Math|Vector|SelectVector (Math|Vector|Normalize (* (Math|Vector|CrossProduct (.ImpactNormal (Collision|BreakHitResult _outhit)) (Transformation|GetActorRightVector)) -1.0)) (Transformation|GetActorForwardVector) _returnvalue_2))) (* (.Z (Math|Vector|BreakVector (Math|Vector|SelectVector (Math|Vector|Normalize (* (Math|Vector|CrossProduct (.ImpactNormal (Collision|BreakHitResult _outhit)) (Transformation|GetActorRightVector)) -1.0)) (Transformation|GetActorForwardVector) _returnvalue_2))) 3.0)) (* (Variables|Default|GetAddForwardVelocityOnJump) _returnvalue_3)) true 0.0 true "MOVE_Falling" false)
        (Class|PrimalCharacter|PlayAnimEx "/Game/PrimalEarth/Dinos/Troodon/Animations/Troodon-Jump-In_Montage.Troodon-Jump-In_Montage" 1.0 "None" true true false false)
        (else
          (|CallParentFunction :!label _label))))
    (:Is%20Not%20Valid
      (goto _label))))

(fn BlueprintAdjustOutputDamage
  (params (AttackIndex :type Integer) (OriginalDamageAmount :type Float%20%28single-precision%29) (HitActor :type Actor%20Object%20Reference))
  (bind _attackinfos (Variables|Default|GetAttackInfos))
  (bind _item (Utilities|Array|Get(acopy) _attackinfos AttackIndex))
  (bind (_attackname _attackweight _attackrange _minattackrange _activateattackrange _attackinterval _bhighqualityattack _bskipuntamed _bskiptamed _bonlyonwilddinos _bpreventwhenencumbered _bridingonlyallowonground _bridingonlyallowwhileflying _bonlyusewithplayersorriders _bonlyusewithplayers _bpreventwhenswimming _bpreventwheninsufficientstamina _bskiponflyers _bskipai _bpreventonfemale _bpreventonmale _bpreventwhendinocarrying _buseblueprintcanriderattack _brequireswalking _attackstatusstarted _battackstopsmovement _battackwithjump _blocationbasedattack _bdropcarriedcharacter _bcancelanddropifcarriedcharacter _bpreventattackwhilerunning _forceupdateinrange _forceupdatemeshself _busesecondaryanimationinair _buseblueprintcanattack _buseblueprintadjustoutputdamage _bdisablerunningwhenattacking _bkeepexecutingwhenacquiringtarget _bpreventwithrider _baiforceattackdotproductcheck _binstantlyharvestcorpse _baddpawnvelocitytoprojectile _battackstopsrotation _btamedaispecialattack _bpreventwhencarryingexplosive _ballowwhenanimationpreventsinput _childstateindexes _attackwithjumpchance _lastattacktime _riderlastattacktime _attackselectionexpirationtime _attackselectiontime _attackrotationrangedegrees _attackrotationgroundspeedmultiplier _attackrotationrate _meleeswingsockets _rangedsocket _meleedamageamount _meleedamageimpulse _meleeswingradius _meleedamagetype) (Utilities|Struct|BreakDinoAttackInfo _item))
  (bind _asprimaldinocharacter (Utilities|Casting|CastToPrimalDinoCharacter HitActor)
    (:then
      (Variables|Default|SetTargetHasARider (Variables|/Script/ShooterGame.PrimalDinoCharacter|GetbHasRider _asprimaldinocharacter))
      (bind _asdino_aicontroller_bp_c (Utilities|Casting|CastToDino_AIController_BP (Class|Actor|GetCharacterController _asprimaldinocharacter))
        (:then
          (bind _returnvalue (Class|PrimalDinoAIController|GetTarget _asdino_aicontroller_bp_c))
          (Utilities|IsValid _returnvalue
            (:Is%20Valid
              (Variables|Default|SetTargetHasATarget true))
            (:Is%20Not%20Valid
              (Variables|Default|SetTargetHasATarget false))))
        (:CastFailed
          _)))
    (:CastFailed
      _))
  (return _meleedamagetype _meleedamageimpulse OriginalDamageAmount))

(fn BPonMovementModeChangedNotify
  (bind _charactermovement (Variables|Character|GetCharacterMovement))
  (switch Utilities|FlowControl|Switch|SwitchonEMovementMode (Variables|/Script/Engine.CharacterMovementComponent|GetMovementMode _charactermovement)
    (:MOVE_Walking
      (if (Variables|Default|GetbStopMovementOnLanding)
        (Components|Movement|StopMovementImmediately _charactermovement)
        (Variables|Default|SetbStopMovementOnLanding false)))
    (:MOVE_Swimming
      (Variables|Default|SetbStopMovementOnLanding false))))

(fn BlueprintDrawFloatingHUD
  (params (HUD :type Shooter%20HUD%20Object%20Reference) (CenterX :type Float%20%28single-precision%29) (CenterY :type Float%20%28single-precision%29) (DrawScale :type Float%20%28single-precision%29))
  (for (_array_element _array_index) (Variables|Sonar|GetSonarDisplayTimes)
    (if (not (Class|VictoryCore|IsTimeSince (Class|Actor|GetWorld) _array_element (Variables|Sonar|GetSonarDisplayTimeLength) true))
      (switch int _array_index
        (:0
          (CallFunction|DrawSonarPoints _array_index (Variables|Sonar|GetSonarPointsType0) HUD))
        (:1
          (CallFunction|DrawSonarPoints _array_index (Variables|Sonar|GetSonarPointsType1) HUD))
        (:2
          (CallFunction|DrawSonarPoints _array_index (Variables|Sonar|GetSonarPointsType2) HUD))
        (:3
          (CallFunction|DrawSonarPoints _array_index (Variables|Sonar|GetSonarPointsType3) HUD))))))

(fn DrawSonarPoints
  (params (SonarType :type Integer) (SonarPoints :type Array%20of%20Vectors) (TheHUD :type Shooter%20HUD%20Object%20Reference))
  (bind _returnvalue (Utilities|Time|GetGameTimeinSeconds))
  (bind _returnvalue_2 (Math|Conversions|ToFloat(Integer) _returnvalue))
  (bind _returnvalue_3 (* _returnvalue_2 4.0))
  (bind _returnvalue_4 (Math|Trig|Sin(Radians) _returnvalue_3))
  (bind _returnvalue_5 (Math|Float|Absolute(Float) _returnvalue_4))
  (bind _returnvalue_6 (* _returnvalue_5 0.5))
  (bind _returnvalue_7 (+ _returnvalue_6 1.25))
  (bind _returnvalue_8 (* _returnvalue_7 32.0))
  (bind _returnvalue_9 (* _returnvalue_8 0.5))
  (for _array_element SonarPoints
    (bind _returnvalue_10 (Class|VictoryCore|BPProjectWorldtoScreenPosition (Math|Vector|MakeVector (.X (Math|Vector|BreakVector _array_element)) (.Y (Math|Vector|BreakVector _array_element)) (+ (.Z (Math|Vector|BreakVector _array_element)) 5e+01)) (Game|Player|GetOwningPlayerController TheHUD)))
    (Canvas|DrawTexture TheHUD (Utilities|Array|Get(acopy) (Variables|Sonar|GetSonarIcons) SonarType) (- (.X (Math|Vector2D|BreakVector2D _returnvalue_10)) _returnvalue_9) (- (.Y (Math|Vector2D|BreakVector2D _returnvalue_10)) _returnvalue_9) _returnvalue_8 _returnvalue_8 0.0 0.0 1.0 1.0)))

(fn BPGetMultiUseEntries
  (params (ForPC :type Player%20Controller%20Object%20Reference) (MultiUseEntries :type Array%20of%20Multi%20Use%20Entry%20Structures))
  (bind _color (Math|Color|MakeColor 40 255 255 255))
  (bind _color_2 (Math|Color|MakeColor 200 200 200 200))
  (bind _basesonarcooldown (Variables|Sonar|GetBaseSonarCooldown))
  (bind _currentsonarcooldownlevel (Variables|Sonar|GetCurrentSonarCooldownLevel))
  (bind _sonarcooldownreductionperlevel (Variables|Sonar|GetSonarCooldownReductionPerLevel))
  (bind _returnvalue (* _currentsonarcooldownlevel _sonarcooldownreductionperlevel))
  (bind _returnvalue_2 (- _basesonarcooldown _returnvalue))
  (bind _returnvalue_3 (Math|Float|Max(Float) _returnvalue_2 2.0))
  (Utilities|FlowControl|Sequence
    (:then_0
      (if (and (Class|PrimalCharacter|BPIsConscious) (== (Variables|/Script/Engine.Actor|GetTargetingTeam ForPC) (Variables|Default|GetTargetingTeam)))
        (bind _returnvalue_4 (Class|VictoryCore|StaticGetTimeSince (Class|Actor|GetWorld) (Variables|Sonar|GetLastTimeSonarWasUsed)))
        (Utilities|Array|Add MultiUseEntries (Utilities|Struct|MakeMultiUseEntry 0 "Scout - Players & Tames" 983940 -1 false (not (>= _returnvalue_4 _returnvalue_3)) false false false false false false false true 2 _color_2 _color))
        (Utilities|Array|Add MultiUseEntries (Utilities|Struct|MakeMultiUseEntry 0 "Scout - Players" 983941 -2 false (not (>= _returnvalue_4 _returnvalue_3)) false false false false false false false true 2 _color_2 _color))
        (Utilities|Array|Add MultiUseEntries (Utilities|Struct|MakeMultiUseEntry 0 "Scout- Traps" 983942 -3 false (not (>= _returnvalue_4 _returnvalue_3)) false false false false false false false true 2 _color_2 _color))
        (Utilities|Array|Add MultiUseEntries (Utilities|Struct|MakeMultiUseEntry 0 "Scout- Wild Creatures" 983943 -4 false (not (>= _returnvalue_4 _returnvalue_3)) false false false false false false false true 2 _color_2 _color))
        (Utilities|Array|Add MultiUseEntries (Utilities|Struct|MakeMultiUseEntry 0 (Utilities|String|ToString(Text) (Utilities|Text|FormatText "Scout - Range {range} - Recharge Time {recharge} sec" (Utilities|Text|ToText(Float) (+ (* (Variables|Sonar|GetCurrentSonarRangeLevel) (Variables|Sonar|GetSonarRangePerLevel)) (Variables|Sonar|GetBaseSonarRange)) "HalfToEven") (Utilities|Text|ToText(Float) _returnvalue_3 "HalfToEven"))) 983944 -9 false (not (>= _returnvalue_4 _returnvalue_3)) false false false false false false true true 0 _color_2 _color))
        (Utilities|Array|Add MultiUseEntries (Utilities|Struct|MakeMultiUseEntry 0 "Back" 983945 -10 false false false false false false false false true true 2 "(B=175,G=175,R=175,A=255)" _color))
        (Utilities|Array|Add MultiUseEntries (Utilities|Struct|MakeMultiUseEntry 0 "Back" 983946 -11 false false false false false false false false true true 3 "(B=175,G=175,R=175,A=255)" _color))
        (bind _returnvalue_5 (Class|PrimalCharacterStatusComponent|HasExperienceforLevelUp (Variables|Default|GetMyCharacterStatusComponent)))
        (Utilities|Array|Add MultiUseEntries (Utilities|Struct|MakeMultiUseEntry 0 "Consume Level Up to Improve Scouting" 983947 -12 false (not _returnvalue_5) false false false false false false true true 0 _color_2 _color))
        (Utilities|Array|Add MultiUseEntries (Utilities|Struct|MakeMultiUseEntry 0 (Utilities|String|ToString(Text) (Utilities|Text|FormatText "Range Level {range} - Recharge Level {recharge}" (Utilities|Text|ToText(Integer) (Variables|Sonar|GetCurrentSonarRangeLevel)) (Utilities|Text|ToText(Integer) (Variables|Sonar|GetCurrentSonarCooldownLevel)))) 983948 1 false false false false false false false false false false 3))
        (Utilities|Array|Add MultiUseEntries (Utilities|Struct|MakeMultiUseEntry 0 "Improve Scouting Range" 983949 -1 false (not _returnvalue_5) false false false false false false false true 3 _color_2 _color))
        (Utilities|Array|Add MultiUseEntries (Utilities|Struct|MakeMultiUseEntry 0 "Improve Scouting Recharge Rate" 983950 -2 false (not _returnvalue_5) false false false false false false false true 3 _color_2 _color))))
    (:then_1
      (return MultiUseEntries))))

(fn BPTryMultiUse
  (params (ForPC :type Player%20Controller%20Object%20Reference) (UseIndex :type Integer))
  (Utilities|FlowControl|Sequence
    (:then_0
      (switch int UseIndex
        (:983940
          (Variables|Sonar|SetSonarMode 0 false)
          (Class|PrimalCharacter|PlayAnimEx "/Game/PrimalEarth/Dinos/Troodon/Animations/Troodon-Sniff_Montage.Troodon-Sniff_Montage" 1.0 "None" true true false false :!label _label)
          (Variables|Sonar|SetLastTimeSonarWasUsed (Utilities|Time|GetGameTimeinSeconds))
          (CallFunction|NetUpdateLastTimeSonarUsed))
        (:983941
          (Variables|Sonar|SetSonarMode 1 false)
          (goto _label))
        (:983942
          (Variables|Sonar|SetSonarMode 2 false)
          (goto _label))
        (:983943
          (Variables|Sonar|SetSonarMode 3 false)
          (goto _label))
        (:983949
          (CallFunction|LevelUpSonar))
        (:983950
          (CallFunction|LevelUpSonar 1))))
    (:then_1
      (return true))))

(fn DoSonar
  (params (SonarType :type Integer))
  (bind _sonarvecs (LocalVariables|GetSonarVecs))
  (bind _returnvalue (Class|VictoryCore|ServerOctreeOverlapActorsBitMask (Class|Actor|GetWorld) (Transformation|GetActorLocation) (+ (* (Variables|Sonar|GetCurrentSonarRangeLevel) (Variables|Sonar|GetSonarRangePerLevel)) (Variables|Sonar|GetBaseSonarRange)) (Utilities|Select :Index SonarType :Option%200 32772 :Option%201 4 :Option%202 67108864 :Option%203 8)))
  (bind _array_element (Utilities|Array|ForEachLoopwithBreak _returnvalue :!label _label)
    (:LoopBody
      (if (and (or (!= SonarType 3) (< (Variables|/Script/Engine.Actor|GetTargetingTeam _array_element) 50000)) (!= (Variables|/Script/Engine.Actor|GetTargetingTeam _array_element) (Variables|Default|GetTargetingTeam)))
        (Utilities|Array|Add _sonarvecs (Transformation|GetActorLocation _array_element))
        (if (> (Utilities|Array|Length _sonarvecs) 29)
          (goto _label Break))))
    (:Completed
      (CallFunction|NetDisplaySonar SonarType _sonarvecs))))

(fn BPClientDoMultiUse
  (params (ForPC :type Player%20Controller%20Object%20Reference) (ClientUseIndex :type Integer))
  (bind _asshooterplayercontroller (Utilities|Casting|CastToShooterPlayerController ForPC))
  (switch int ClientUseIndex
    (:983944
      (Class|ShooterPlayerController|SetMultiUseWheelCategory _asshooterplayercontroller 2))
    (:983945
      (Class|ShooterPlayerController|SetMultiUseWheelCategory _asshooterplayercontroller 0 :!label _label))
    (:983946
      (goto _label))
    (:983947
      (Class|ShooterPlayerController|SetMultiUseWheelCategory _asshooterplayercontroller 3))))

(fn LevelUpSonar
  (params (Selector :type Integer))
  (bind _mycharacterstatuscomponent (Variables|Default|GetMyCharacterStatusComponent))
  (switch int Selector
    (:0
      (Variables|Sonar|SetCurrentSonarRangeLevel (+ (Variables|Sonar|GetCurrentSonarRangeLevel) 1) false))
    (:1
      (Variables|Sonar|SetCurrentSonarCooldownLevel (+ (Variables|Sonar|GetCurrentSonarCooldownLevel) 1) false)))
  (Class|PrimalCharacterStatusComponent|SetExtraCharacterLevel _mycharacterstatuscomponent (+ (Class|PrimalCharacterStatusComponent|GetExtraCharacterLevel _mycharacterstatuscomponent) 1))
  (Class|PrimalCharacter|PlayAnimEx (Variables|Default|GetBabyCuddledAnimation) 1.0 "None" true false false false))

(fn BPGetAddForwardVelocityonJump
  (return (select (Class|VictoryCore|IsTimeSince (Class|Actor|GetWorld) (Variables|Default|GetLastTimeInSwimming) 0.25 true) 1.0 0.0)))