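; AI controller for the King Leedsichthys mod creature that biases which targets it chooses to attack.
; It overrides targeting desire to scale rafts by a raft aggro multiplier, regardless of recent damage.
; Other targets get a desire of -1 once the Leedsichthys's post-damage aggression window has elapsed, so it pursues them only shortly after being hurt.
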(fn ConstructionScript
  (|CallParentFunction))

(fn BPGetTargetingDesire
  (params (ForTarget :type Actor%20Object%20Reference) (ForTargetingDesireValue :type Float%20%28single-precision%29))
  (LocalVariables|SetRetVal ForTargetingDesireValue)
  (Utilities|Casting|CastToPrimalRaft ForTarget
    (:then
      (LocalVariables|SetRetVal (* ForTargetingDesireValue (Variables|Default|GetRaftAggroMultiplier))))
    (:CastFailed
      (bind _asleedsichthys_character_bp_c (Utilities|Casting|CastToLeedsichthys_Character_BP (Pawn|GetControlledPawn))
        (:then
          (if (Class|VictoryCore|IsTimeSince (Class|Actor|GetWorld _asleedsichthys_character_bp_c) (Variables|/Game/PrimalEarth/Dinos/Leedsichthys/Leedsichthys_Character_BP.Leedsichthys_Character_BP_C|GetLastTimeTookDamage _asleedsichthys_character_bp_c) (Variables|/Game/PrimalEarth/Dinos/Leedsichthys/Leedsichthys_Character_BP.Leedsichthys_Character_BP_C|GetTimeAggressiveAfterDamageTaken _asleedsichthys_character_bp_c) true)
            (LocalVariables|SetRetVal -1.0)))
        (:CastFailed
          _))))
  (return (LocalVariables|GetRetVal)))