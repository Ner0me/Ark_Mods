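; King Archa character Blueprint, an Archaeopteryx-style dino that glides, perches on trees and slows its carrier's falls.
; Unmounted, a blackboard flag scales its falling gravity; when tamed and carried, tick adds upward impulses to the falling carrier.
; A server-routed command toggles that glide, which re-enables on each new fall and overrides air control.
; Tamed wanderers attached to trees periodically gain sap; mounting or falling unconscious detaches them.
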(event Custom|MultiFinishAttachingToTree
  (params (relLoc :type Vector) (relRot :type Rotator))
  (Transformation|SetActorRelativeLocation relLoc)
  (Transformation|SetActorRelativeRotation relRot)
  (Animation|PlayAnimMontage "/Game/PrimalEarth/Dinos/Archaeopteryx/Animations/Archaeopteryx-StartPerch_Montage.Archaeopteryx-StartPerch_Montage" 1.0 "None" false))

(fn ConstructionScript
  (|CallParentFunction))

(fn BPGetGravityZScale
  (bind _returnvalue (Pawn|GetController))
  (bind _charactermovement (Variables|Character|GetCharacterMovement))
  (bind _returnvalue_2 (AI|GetBlackboard _returnvalue))
  (LocalVariables|Setret 1.0)
  (Utilities|FlowControl|Sequence
    (:then_0
      (if (Utilities|IsValid _charactermovement)
        (if (Math|Boolean|ANDBoolean (Variables|Default|GetbGlideWhenFalling) (Utilities|Enum|Equal(Enum) (Variables|/Script/Engine.CharacterMovementComponent|GetMovementMode _charactermovement) "MOVE_Falling") (< (.Z (Math|Vector|BreakVector (Variables|/Script/Engine.MovementComponent|GetVelocity _charactermovement))) 0.0))
          (Utilities|IsValid _returnvalue
            (:Is%20Valid
              (Utilities|IsValid _returnvalue_2
                (:Is%20Valid
                  (if (ScalableFloat|GetValueasBool _returnvalue_2 (Utilities|Name|MakeLiteralName "ShouldGlide"))
                    (LocalVariables|Setret (Variables|Default|GetGlideGravityScaleMultiplier))))))))))
    (:then_1
      (return (LocalVariables|Getret)))))

(fn ReceiveTick
  (params (DeltaSeconds :type Float%20%28single-precision%29))
  (bind _mountcharacter (Variables|Default|GetMountCharacter))
  (bind _charactermovement (Variables|/Script/Engine.Character|GetCharacterMovement _mountcharacter))
  (if (Class|PrimalDinoCharacter|BPIsTamed)
    (Utilities|IsValid _mountcharacter
      (:Is%20Valid
        (if (Utilities|Enum|Equal(Enum) (Variables|/Script/Engine.CharacterMovementComponent|GetMovementMode _charactermovement) "MOVE_Falling")
          (if (or (Variables|Default|GetbWasMountedFalling) (not (Ability|HasAuthority)))
            _
            (elif (Variables|Default|GetbPreventGlide)
              (Variables|Default|SetbPreventGlide false)))
          (Variables|Default|SetbWasMountedFalling true)
          (if (< (.Z (Math|Vector|BreakVector (Variables|/Script/Engine.MovementComponent|GetVelocity _charactermovement))) (* (* (Variables|/Script/ShooterGame.PrimalCharacter|GetMaxFallSpeed _mountcharacter) (Variables|Default|GetGlideGravityScaleMultiplier)) -1.0))
            (if (not (Variables|Default|GetbPreventGlide))
              (Physics|AddImpulse _charactermovement (Math|Vector|MakeVector 0.0 0.0 (* DeltaSeconds 1.05e+03)) true 0.55)))
          (else
            (Variables|Default|SetbWasMountedFalling false))))
      (:Is%20Not%20Valid
        (if (Variables|Default|GetbEnableTamedWandering)
          (if (Utilities|IsValid (Transformation|GetAttachParent (VehicleSound|GetRootComponent)))
            (if (and (< (Class|PrimalCharacterStatusComponent|BPGetPercentStatusValue (Variables|Default|GetMyCharacterStatusComponent) "Weight") 1.0) (Ability|HasAuthority))
              (Variables|Default|SetTimeSpentOnTreeCache (+ (Variables|Default|GetTimeSpentOnTreeCache) DeltaSeconds))
              (if (> (Variables|Default|GetTimeSpentOnTreeCache) (Variables|Default|GetIntervalGiveSapOnTree))
                (Variables|Default|SetTimeSpentOnTreeCache 0.0)
                (CallFunction|GiveSap)))))))))

(fn BPonClearMountedDino
  (bind _returnvalue (Pawn|GetController))
  (Utilities|IsValid _returnvalue
    (:Is%20Valid
      (bind _asprimaldinoaicontroller (Utilities|Casting|CastToPrimalDinoAIController _returnvalue))
      (AI|RunBehaviorTree _asprimaldinoaicontroller (Variables|/Script/ShooterGame.PrimalDinoAIController|GetNoEnemyTree _asprimaldinoaicontroller)))))

(fn BPonSetMountedDino
  (bind _returnvalue (Pawn|GetController))
  (Utilities|IsValid (VehicleSound|GetRootComponent)
    (:Is%20Valid
      (Class|Actor|DetachRootComponentfromParent true))
    (:Is%20Not%20Valid
      _))
  (Utilities|IsValid _returnvalue
    (:Is%20Valid
      (bind _asprimaldinoaicontroller (Utilities|Casting|CastToPrimalDinoAIController _returnvalue))
      (Class|PrimalDinoAIController|StopBrainComponent _asprimaldinoaicontroller "Mounted"))))

(fn BPonAttachmentReplication
  (bind _returnvalue (VehicleSound|GetRootComponent))
  (bind _attachmentreplication (Variables|Default|GetAttachmentReplication))
  (bind _attachcomponent (Utilities|Struct|BreakRepAttachment _attachmentreplication))
  (LocalVariables|Setret false)
  (Utilities|FlowControl|Sequence
    (:then_0
      (Utilities|IsValid _returnvalue
        (:Is%20Valid
          (if (!= (Transformation|GetAttachParent _returnvalue) 0)
            (Utilities|IsValid _attachcomponent
              (:Is%20Valid
                (Utilities|Casting|CastToHierarchicalInstancedStaticMeshComponent _attachcomponent)
                (LocalVariables|Setret true)))
            (else
              (LocalVariables|Setret true))))))
    (:then_1
      (return (LocalVariables|Getret)))))

(fn GiveSap
  (Class|PrimalInventoryComponent|BPIncrementItemTemplateQuantity (Variables|Default|GetMyInventoryComponent) (Variables|Default|GetSapItemClass) 1 true false true false false false))

(fn BPCharacterSleeped
  (if (Ability|HasAuthority)
    (if (Utilities|IsValid (Transformation|GetAttachParent (VehicleSound|GetRootComponent)))
      (Class|Actor|DetachRootComponentfromParent true)
      (Class|PrimalCharacter|OnDetachedfromCharacter)
      (Transformation|SetActorRotation "0, 0, 0")
      (Pawn|Components|CharacterMovement|SetMovementMode (Variables|Character|GetCharacterMovement) "MOVE_Falling" 0))))

(fn HandleMountedDinoAction
  (params (PC :type Shooter%20Player%20Controller%20Object%20Reference))
  (Class|PlayerController|ClientSendNetExecCommandtoServer PC self "ToggleGlide" (Utilities|Struct|MakeBPNetExecParams) true))

(fn OnRepBPreventGlide)

(fn BPServerHandleNetExecCommand
  (params (FromPC :type Player%20Controller%20Object%20Reference) (CommandName :type Name :default "None") (ExecParams :type BP%20Net%20Exec%20Params%20Structure%20%28by%20ref%29))
  (Utilities|FlowControl|Sequence
    (:then_0
      (if (Utilities|Name|Equal(Name) CommandName "ToggleGlide")
        (bind _asshooterplayercontroller (Utilities|Casting|CastToShooterPlayerController FromPC))
        (Utilities|IsValid (Class|ShooterPlayerController|GetPlayerCharacter _asshooterplayercontroller)
          (:Is%20Valid
            (if (== (Class|ShooterPlayerController|GetPlayerCharacter _asshooterplayercontroller) (Variables|Default|GetMountCharacter))
              (Variables|Default|SetbPreventGlide (not (Variables|Default|GetbPreventGlide)))
              (Networking|ForceNetUpdate))))))
    (:then_1
      (return true))))

(fn DoOverrideMountedAirControl
  (params (AirControlIn :type Float%20%28single-precision%29))
  (return (select (Variables|Default|GetbPreventGlide) AirControlIn (Variables|Default|GetMountedAirControl))))