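; King Liopleurodon creature Blueprint for an ARK mod, granting a magic buff to nearby player pawns on its team.
; RefreshMagicBuffTimers finds pawns through a server octree query and applies the buff, and runs when a rider is set.
; Taming enables the server timer flag and magic particle, both shut off on death, while a helper computes remaining tame time from TameTime.
; An anim notify spawns a whirlpool spin effect, skipped on dedicated servers.
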(event Custom|OnDied_ClearParticles
  (params (DiedCharacter :type Primal%20Character%20Object%20Reference))
  ;[0.02303 0.255 0] Begin play Bind Ondied
  (Components|DestroyComponent (Variables|Default|GetMagicParticle))
  (Variables|Default|SetbUseBPTimerServer false))

(event Custom|RefreshMagicBuffTimers
  ;[0 0.6586 1] Refresh Magic Buff
  (bind _returnvalue (Class|VictoryCore|ServerOctreeOverlapActors (Class|Actor|GetWorld) (Transformation|GetActorLocation) (Variables|Default|GetMagicBuffRadius) "PLAYERPAWNS"))
  (for _array_element _returnvalue
    (bind _asshootercharacter (Utilities|Casting|CastToShooterCharacter _array_element))
    (if (== (Variables|/Script/Engine.Actor|GetTargetingTeam _asshootercharacter) (Variables|Default|GetTargetingTeam))
      (Class|PrimalBuff|StaticAddBuff (Variables|Default|GetMagicBuffClass) _asshootercharacter 0 self false))))

(event Custom|AnimNotify_SpawnSpinEffect
  ;[1 0.09928 0] Spin particle effect
  (if (not (Networking|IsDedicatedServer))
    (Effects|SpawnEmitteratLocation "/Game/PrimalEarth/Effects/Particles/Creatures/Liopleuro/P_Liopleuro_Whirlpool2.P_Liopleuro_Whirlpool2" (Transformation|GetActorLocation) (Transformation|GetActorRotation) true false)))

(event EventBeginPlay
  ;[0.02303 0.255 0] Begin play Bind Ondied
  (EventDispatchers|BindEventtoOnDied (delegate Custom|OnDied_ClearParticles)))

(fn ConstructionScript
  (|CallParentFunction))

(fn BPNotifySetRider
  (params (RiderSetting :type Shooter%20Character%20Object%20Reference))
  (CallFunction|RefreshMagicBuffTimers))

(fn BPSetupTamed
  (params (bWasJustTamed :type Boolean))
  (Variables|Default|SetbUseBPTimerServer true)
  (Components|Activation|Activate (Variables|Default|GetMagicParticle) false))

(fn FindRemainingTameTime
  (Utilities|FlowControl|Sequence
    (:then_0
      (bind _asshootergamestate (Utilities|Casting|CastToShooterGameState (Game|GetGameState)))
      (bind _returnvalue (Class|ShooterGameState|GetNetworkTimeDelta _asshootergamestate (Variables|Local/DoNotEdit|GetTameTime) true))
      (LocalVariables|SetretVal (Math|Float|Max(Float) (Math|Conversions|ToFloat(Integer) _returnvalue) 0.0)))
    (:then_1
      (return (LocalVariables|GetretVal)))))